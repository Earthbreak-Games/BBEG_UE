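; Stage manager Blueprint that streams rooms into a stage as level instances placed at a given transform.
; Room spawning takes the first entry of a randomly chosen Starts or Combat set; the wired DangerousCombat option falls outside the random range.
; Helpers pick random boss and start rooms, but the boss spawn event leaves its level name unconnected and the start helper is not called here.
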(event `InstantiateNewRoom`
  (params (StartTransform :type "Transform Structure"))
  ;[1 1 1] Room Instancing
  (bind _roomtospawn (`self.GetRoomToSpawn`))
  (`LevelStreamingDynamic.LoadLevelInstance` _roomtospawn StartTransform_Location StartTransform_Rotation "" null))

(event `InstantiateNewBossRoom`
  (params (StartTransform :type "Transform Structure"))
  ;[1 1 1] Room Instancing
  (bind _roomtospawn (`self.GetBossRoom`))
  (`LevelStreamingDynamic.LoadLevelInstance` "" StartTransform_Location StartTransform_Rotation "" null))

(fn `GetBossRoom`
  (returns (RoomToSpawn :type String))
  (bind _result (`BlueprintSetLibrary.Set_ToArray` (`self.Boss`)))
  (return (`|GetArrayItem` _result (`KismetMathLibrary.RandomInteger` (`KismetArrayLibrary.Array_Length` _result)))))

(fn `GetRoomToSpawn`
  (returns (RoomToSpawn :type String))
  (bind _result (`BlueprintSetLibrary.Set_ToArray` (select `int` (`KismetMathLibrary.RandomInteger` 2) :`0` (`self.Starts`) :`1` (`self.Combat`) :`2` (`self.DangerousCombat`))))
  (return (`|GetArrayItem` _result)))

(fn `GetStartRoom`
  (returns (RoomToSpawn :type String))
  (bind _result (`BlueprintSetLibrary.Set_ToArray` (`self.Starts`)))
  (return (`|GetArrayItem` _result (`KismetMathLibrary.RandomInteger` (`KismetArrayLibrary.Array_Length` _result)))))

(fn `UserConstructionScript`)