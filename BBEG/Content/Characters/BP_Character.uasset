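; Character Blueprint that handles melee and ranged attack input on top of a parent class.
; Each attack trigger checks through NotInAttackState against the character's current state, starts its MeleeAttack or RangedAttack, then calls Stop.
; The T key prints the current state and calls ResumeInput as a debug aid.
; Disconnected nodes keep experiments with forced movement input and ignoring move input.
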(event `self.ReceiveBeginPlay`
  (`parent.ReceiveBeginPlay`))

(event `self.ReceiveTick`
  (params (DeltaSeconds :type "Float (single-precision)")))

(event `self.EI_TriggerMelee`
  (`self.Not in attack state`)
  (`/Game/Blueprints/Attacks/Attack.AttackStart` (`self.MeleeAttack`))
  (`self.Stop` :!label _label))

(event `self.EI_TriggerRanged`
  (`self.Not in attack state`)
  (`/Game/Blueprints/Attacks/Attack.AttackStart` (`self.RangedAttack`))
  (goto _label))

(event `Key|T`
  (params (Key :type "Key Structure"))
  (:`Pressed`
    (`self.Print State`)
    (`self.ResumeInput`)))

(fn `Print State`
  (bind _returnvalue (`self.GetState`))
  (`KismetSystemLibrary.PrintString` (`|GetEnumeratorNameAsString` _returnvalue)))

(fn `UserConstructionScript`)